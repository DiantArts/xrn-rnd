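; Core player controller that requests pawn spawning at startup and links the local player to HUD, chat and abilities.
; Chat messages go to the server, which relays them to every controller's client HUD through a PlayerArray loop macro.
; Skillbar inputs send the slot's ability class to the game state via server events while starting the cast bar locally.
; It also spawns client-side abilities and forwards cast cancels and interrupts.
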(event Custom|SR_SpawnPlayer
  (bind _bp_gm_basesetup (Utilities|GetGMBaseSetup))
  (Default|SpawnPlayer _bp_gm_basesetup self))

(event EventBeginPlay
  (bind _asbp_core_gs (Utilities|Casting|CastToBP_Core_GS (Game|GetGameState))
    (:then
      (Variables|Default|SetBP_Core_GS _asbp_core_gs)
      (Utilities|IsLocalPlayerController
        (:True
          (CallFunction|SRSpawnPlayer)
          (bind _bp_core_hud (Utilities|GetBPCoreHUD 1e+01)
            (:Success
              (Variables|Default|SetBP_Core_HUD _bp_core_hud))))))
    (:CastFailed
      (CallFunction|PrintError "BP_Core_PC" "Failed to cast GS to BP_Core_GS"))))

(event Custom|SR_SubmitMessage
  (params (PlayerName :type Text) (ChatMessage :type Text))
  ;[1 1 1] Chat
  (bind _bp_core_pc (Utilities|ForEachPlayerController)
    (:Loop%20Body
      (CallFunction|OCUpdateChat _bp_core_pc PlayerName ChatMessage))))

(event Custom|OC_UpdateChat
  (params (PlayerName :type Text) (ChatMessage :type Text))
  ;[1 1 1] Chat
  (Default|UpdateChat (Variables|Default|GetBP_Core_HUD) PlayerName ChatMessage))

(event Input|ActionEvents|InputActionstartTyping
  (params (Key :type Key%20Structure))
  ;[1 1 1] Chat
  (:Pressed
    (bind _bp_core_hud (Variables|Default|GetBP_Core_HUD)
      (:then
        (Default|StartTyping _bp_core_hud))
      (:else))))

(event Input|ActionEvents|InputActionskillbar-1
  (params (Key :type Key%20Structure))
  (:Pressed
    (CallFunction|UseAbility (Variables|/Game/xrn/Widgets/UI/ActionBar/WB_ActionBarSlot.WB_ActionBarSlot_C|GetAbilityClass (Variables|/Game/xrn/Widgets/UI/ActionBar/WB_ActionBar.WB_ActionBar_C|Getslot_skillbar-1 (Variables|/Game/xrn/Widgets/UI/WB_HUD.WB_HUD_C|GetWB_ActionBar (Variables|/Game/xrn/Blueprints/Core/BP_Core_HUD.BP_Core_HUD_C|GetWB_HUD (Variables|Default|GetBP_Core_HUD))))) (Pawn|GetControlledPawn))))

(event Input|ActionEvents|InputActionskillbar-6
  (params (Key :type Key%20Structure))
  (:Pressed
    (CallFunction|UseAbility (Variables|/Game/xrn/Widgets/UI/ActionBar/WB_ActionBarSlot.WB_ActionBarSlot_C|GetAbilityClass (Variables|/Game/xrn/Widgets/UI/ActionBar/WB_ActionBar.WB_ActionBar_C|Getslot_skillbar-6 (Variables|/Game/xrn/Widgets/UI/WB_HUD.WB_HUD_C|GetWB_ActionBar (Variables|/Game/xrn/Blueprints/Core/BP_Core_HUD.BP_Core_HUD_C|GetWB_HUD (Variables|Default|GetBP_Core_HUD))))) (Pawn|GetControlledPawn))))

(event Input|ActionEvents|InputActionskillbar-7
  (params (Key :type Key%20Structure))
  (:Pressed
    (CallFunction|UseAbility (Variables|/Game/xrn/Widgets/UI/ActionBar/WB_ActionBarSlot.WB_ActionBarSlot_C|GetAbilityClass (Variables|/Game/xrn/Widgets/UI/ActionBar/WB_ActionBar.WB_ActionBar_C|Getslot_skillbar-7 (Variables|/Game/xrn/Widgets/UI/WB_HUD.WB_HUD_C|GetWB_ActionBar (Variables|/Game/xrn/Blueprints/Core/BP_Core_HUD.BP_Core_HUD_C|GetWB_HUD (Variables|Default|GetBP_Core_HUD))))) (Pawn|GetControlledPawn))))

(event Input|ActionEvents|InputActionskillbar-8
  (params (Key :type Key%20Structure))
  (:Pressed
    (CallFunction|UseAbility (Variables|/Game/xrn/Widgets/UI/ActionBar/WB_ActionBarSlot.WB_ActionBarSlot_C|GetAbilityClass (Variables|/Game/xrn/Widgets/UI/ActionBar/WB_ActionBar.WB_ActionBar_C|Getslot_skillbar-8 (Variables|/Game/xrn/Widgets/UI/WB_HUD.WB_HUD_C|GetWB_ActionBar (Variables|/Game/xrn/Blueprints/Core/BP_Core_HUD.BP_Core_HUD_C|GetWB_HUD (Variables|Default|GetBP_Core_HUD))))) (Pawn|GetControlledPawn))))

(event Input|ActionEvents|InputActionskillbar-9
  (params (Key :type Key%20Structure))
  (:Pressed
    (CallFunction|UseAbility (Variables|/Game/xrn/Widgets/UI/ActionBar/WB_ActionBarSlot.WB_ActionBarSlot_C|GetAbilityClass (Variables|/Game/xrn/Widgets/UI/ActionBar/WB_ActionBar.WB_ActionBar_C|Getslot_skillbar-9 (Variables|/Game/xrn/Widgets/UI/WB_HUD.WB_HUD_C|GetWB_ActionBar (Variables|/Game/xrn/Blueprints/Core/BP_Core_HUD.BP_Core_HUD_C|GetWB_HUD (Variables|Default|GetBP_Core_HUD))))) (Pawn|GetControlledPawn))))

(event Input|ActionEvents|InputActionskillbar-10
  (params (Key :type Key%20Structure))
  (:Pressed
    (CallFunction|UseAbility (Variables|/Game/xrn/Widgets/UI/ActionBar/WB_ActionBarSlot.WB_ActionBarSlot_C|GetAbilityClass (Variables|/Game/xrn/Widgets/UI/ActionBar/WB_ActionBar.WB_ActionBar_C|Getslot_skillbar-10 (Variables|/Game/xrn/Widgets/UI/WB_HUD.WB_HUD_C|GetWB_ActionBar (Variables|/Game/xrn/Blueprints/Core/BP_Core_HUD.BP_Core_HUD_C|GetWB_HUD (Variables|Default|GetBP_Core_HUD))))) (Pawn|GetControlledPawn))))

(event Input|ActionEvents|InputActionskillbar-11
  (params (Key :type Key%20Structure))
  (:Pressed
    (CallFunction|UseAbility (Variables|/Game/xrn/Widgets/UI/ActionBar/WB_ActionBarSlot.WB_ActionBarSlot_C|GetAbilityClass (Variables|/Game/xrn/Widgets/UI/ActionBar/WB_ActionBar.WB_ActionBar_C|Getslot_skillbar-11 (Variables|/Game/xrn/Widgets/UI/WB_HUD.WB_HUD_C|GetWB_ActionBar (Variables|/Game/xrn/Blueprints/Core/BP_Core_HUD.BP_Core_HUD_C|GetWB_HUD (Variables|Default|GetBP_Core_HUD))))) (Pawn|GetControlledPawn))))

(event Input|ActionEvents|InputActionskillbar-12
  (params (Key :type Key%20Structure))
  (:Pressed
    (CallFunction|UseAbility (Variables|/Game/xrn/Widgets/UI/ActionBar/WB_ActionBarSlot.WB_ActionBarSlot_C|GetAbilityClass (Variables|/Game/xrn/Widgets/UI/ActionBar/WB_ActionBar.WB_ActionBar_C|Getslot_skillbar-12 (Variables|/Game/xrn/Widgets/UI/WB_HUD.WB_HUD_C|GetWB_ActionBar (Variables|/Game/xrn/Blueprints/Core/BP_Core_HUD.BP_Core_HUD_C|GetWB_HUD (Variables|Default|GetBP_Core_HUD))))) (Pawn|GetControlledPawn))))

(event Input|ActionEvents|InputActionskillbar-13
  (params (Key :type Key%20Structure))
  (:Pressed
    (CallFunction|UseAbility (Variables|/Game/xrn/Widgets/UI/ActionBar/WB_ActionBarSlot.WB_ActionBarSlot_C|GetAbilityClass (Variables|/Game/xrn/Widgets/UI/ActionBar/WB_ActionBar.WB_ActionBar_C|Getslot_skillbar-13 (Variables|/Game/xrn/Widgets/UI/WB_HUD.WB_HUD_C|GetWB_ActionBar (Variables|/Game/xrn/Blueprints/Core/BP_Core_HUD.BP_Core_HUD_C|GetWB_HUD (Variables|Default|GetBP_Core_HUD))))) (Pawn|GetControlledPawn))))

(event Input|ActionEvents|InputActionskillbar-14
  (params (Key :type Key%20Structure))
  (:Pressed
    (CallFunction|UseAbility (Variables|/Game/xrn/Widgets/UI/ActionBar/WB_ActionBarSlot.WB_ActionBarSlot_C|GetAbilityClass (Variables|/Game/xrn/Widgets/UI/ActionBar/WB_ActionBar.WB_ActionBar_C|Getslot_skillbar-14 (Variables|/Game/xrn/Widgets/UI/WB_HUD.WB_HUD_C|GetWB_ActionBar (Variables|/Game/xrn/Blueprints/Core/BP_Core_HUD.BP_Core_HUD_C|GetWB_HUD (Variables|Default|GetBP_Core_HUD))))) (Pawn|GetControlledPawn))))

(event Input|ActionEvents|InputActionskillbar-15
  (params (Key :type Key%20Structure))
  (:Pressed
    (CallFunction|UseAbility (Variables|/Game/xrn/Widgets/UI/ActionBar/WB_ActionBarSlot.WB_ActionBarSlot_C|GetAbilityClass (Variables|/Game/xrn/Widgets/UI/ActionBar/WB_ActionBar.WB_ActionBar_C|Getslot_skillbar-15 (Variables|/Game/xrn/Widgets/UI/WB_HUD.WB_HUD_C|GetWB_ActionBar (Variables|/Game/xrn/Blueprints/Core/BP_Core_HUD.BP_Core_HUD_C|GetWB_HUD (Variables|Default|GetBP_Core_HUD))))) (Pawn|GetControlledPawn))))

(event Input|ActionEvents|InputActionskillbar-16
  (params (Key :type Key%20Structure))
  (:Pressed
    (CallFunction|UseAbility (Variables|/Game/xrn/Widgets/UI/ActionBar/WB_ActionBarSlot.WB_ActionBarSlot_C|GetAbilityClass (Variables|/Game/xrn/Widgets/UI/ActionBar/WB_ActionBar.WB_ActionBar_C|Getslot_skillbar-16 (Variables|/Game/xrn/Widgets/UI/WB_HUD.WB_HUD_C|GetWB_ActionBar (Variables|/Game/xrn/Blueprints/Core/BP_Core_HUD.BP_Core_HUD_C|GetWB_HUD (Variables|Default|GetBP_Core_HUD))))) (Pawn|GetControlledPawn))))

(event Input|ActionEvents|InputActionskillbar-17
  (params (Key :type Key%20Structure))
  (:Pressed
    (CallFunction|UseAbility (Variables|/Game/xrn/Widgets/UI/ActionBar/WB_ActionBarSlot.WB_ActionBarSlot_C|GetAbilityClass (Variables|/Game/xrn/Widgets/UI/ActionBar/WB_ActionBar.WB_ActionBar_C|Getslot_skillbar-17 (Variables|/Game/xrn/Widgets/UI/WB_HUD.WB_HUD_C|GetWB_ActionBar (Variables|/Game/xrn/Blueprints/Core/BP_Core_HUD.BP_Core_HUD_C|GetWB_HUD (Variables|Default|GetBP_Core_HUD))))) (Pawn|GetControlledPawn))))

(event Input|ActionEvents|InputActionskillbar-18
  (params (Key :type Key%20Structure))
  (:Pressed
    (CallFunction|UseAbility (Variables|/Game/xrn/Widgets/UI/ActionBar/WB_ActionBarSlot.WB_ActionBarSlot_C|GetAbilityClass (Variables|/Game/xrn/Widgets/UI/ActionBar/WB_ActionBar.WB_ActionBar_C|Getslot_skillbar-18 (Variables|/Game/xrn/Widgets/UI/WB_HUD.WB_HUD_C|GetWB_ActionBar (Variables|/Game/xrn/Blueprints/Core/BP_Core_HUD.BP_Core_HUD_C|GetWB_HUD (Variables|Default|GetBP_Core_HUD))))) (Pawn|GetControlledPawn))))

(event Input|ActionEvents|InputActionskillbar-19
  (params (Key :type Key%20Structure))
  (:Pressed
    (CallFunction|UseAbility (Variables|/Game/xrn/Widgets/UI/ActionBar/WB_ActionBarSlot.WB_ActionBarSlot_C|GetAbilityClass (Variables|/Game/xrn/Widgets/UI/ActionBar/WB_ActionBar.WB_ActionBar_C|Getslot_skillbar-19 (Variables|/Game/xrn/Widgets/UI/WB_HUD.WB_HUD_C|GetWB_ActionBar (Variables|/Game/xrn/Blueprints/Core/BP_Core_HUD.BP_Core_HUD_C|GetWB_HUD (Variables|Default|GetBP_Core_HUD))))) (Pawn|GetControlledPawn))))

(event Input|ActionEvents|InputActionskillbar-20
  (params (Key :type Key%20Structure))
  (:Pressed
    (CallFunction|UseAbility (Variables|/Game/xrn/Widgets/UI/ActionBar/WB_ActionBarSlot.WB_ActionBarSlot_C|GetAbilityClass (Variables|/Game/xrn/Widgets/UI/ActionBar/WB_ActionBar.WB_ActionBar_C|Getslot_skillbar-20 (Variables|/Game/xrn/Widgets/UI/WB_HUD.WB_HUD_C|GetWB_ActionBar (Variables|/Game/xrn/Blueprints/Core/BP_Core_HUD.BP_Core_HUD_C|GetWB_HUD (Variables|Default|GetBP_Core_HUD))))) (Pawn|GetControlledPawn))))

(event Input|ActionEvents|InputActionskillbar-2
  (params (Key :type Key%20Structure))
  (:Pressed
    (CallFunction|UseAbility (Variables|/Game/xrn/Widgets/UI/ActionBar/WB_ActionBarSlot.WB_ActionBarSlot_C|GetAbilityClass (Variables|/Game/xrn/Widgets/UI/ActionBar/WB_ActionBar.WB_ActionBar_C|Getslot_skillbar-2 (Variables|/Game/xrn/Widgets/UI/WB_HUD.WB_HUD_C|GetWB_ActionBar (Variables|/Game/xrn/Blueprints/Core/BP_Core_HUD.BP_Core_HUD_C|GetWB_HUD (Variables|Default|GetBP_Core_HUD))))) (Pawn|GetControlledPawn))))

(event Input|ActionEvents|InputActionskillbar-3
  (params (Key :type Key%20Structure))
  (:Pressed
    (CallFunction|UseAbility (Variables|/Game/xrn/Widgets/UI/ActionBar/WB_ActionBarSlot.WB_ActionBarSlot_C|GetAbilityClass (Variables|/Game/xrn/Widgets/UI/ActionBar/WB_ActionBar.WB_ActionBar_C|Getslot_skillbar-3 (Variables|/Game/xrn/Widgets/UI/WB_HUD.WB_HUD_C|GetWB_ActionBar (Variables|/Game/xrn/Blueprints/Core/BP_Core_HUD.BP_Core_HUD_C|GetWB_HUD (Variables|Default|GetBP_Core_HUD))))) (Pawn|GetControlledPawn))))

(event Input|ActionEvents|InputActionskillbar-4
  (params (Key :type Key%20Structure))
  (:Pressed
    (CallFunction|UseAbility (Variables|/Game/xrn/Widgets/UI/ActionBar/WB_ActionBarSlot.WB_ActionBarSlot_C|GetAbilityClass (Variables|/Game/xrn/Widgets/UI/ActionBar/WB_ActionBar.WB_ActionBar_C|Getslot_skillbar-4 (Variables|/Game/xrn/Widgets/UI/WB_HUD.WB_HUD_C|GetWB_ActionBar (Variables|/Game/xrn/Blueprints/Core/BP_Core_HUD.BP_Core_HUD_C|GetWB_HUD (Variables|Default|GetBP_Core_HUD))))) (Pawn|GetControlledPawn))))

(event Input|ActionEvents|InputActionskillbar-5
  (params (Key :type Key%20Structure))
  (:Pressed
    (CallFunction|UseAbility (Variables|/Game/xrn/Widgets/UI/ActionBar/WB_ActionBarSlot.WB_ActionBarSlot_C|GetAbilityClass (Variables|/Game/xrn/Widgets/UI/ActionBar/WB_ActionBar.WB_ActionBar_C|Getslot_skillbar-5 (Variables|/Game/xrn/Widgets/UI/WB_HUD.WB_HUD_C|GetWB_ActionBar (Variables|/Game/xrn/Blueprints/Core/BP_Core_HUD.BP_Core_HUD_C|GetWB_HUD (Variables|Default|GetBP_Core_HUD))))) (Pawn|GetControlledPawn))))

(event Custom|SR_UseAbility
  (params (AbilityClass :type BP%20Ability%20Class%20Reference) (Instigator :type Pawn%20Object%20Reference))
  ;[0 0 0] Use Ability
  (Default|SRSpawnAbility (Variables|Default|GetBP_Core_GS) AbilityClass Instigator))

(event Custom|OC_SpawnClientAbility
  (params (SpawnTransform :type Transform) (AbilityToSpawn :type BP%20Ability%20Class%20Reference) (Instigator :type Pawn%20Object%20Reference))
  ;[0 0 0] Use Ability
  (bind _returnvalue (Game|SpawnActorfromClass AbilityToSpawn SpawnTransform "Undefined" "MultiplyWithRoot" 0 Instigator))
  (Default|ClientBeginCast _returnvalue))

(event Custom|UseAbility
  (params (AbilityClass :type BP%20Ability%20Class%20Reference) (Instigator :type Pawn%20Object%20Reference))
  ;[0 0 0] Use Ability
  (CallFunction|SRUseAbility AbilityClass Instigator)
  ;;[1 1 1] CastBar Animation
  (Default|OnBeginCast (Variables|/Game/xrn/Widgets/UI/WB_HUD.WB_HUD_C|GetWB_CastBar (Variables|/Game/xrn/Blueprints/Core/BP_Core_HUD.BP_Core_HUD_C|GetWB_HUD (Variables|Default|GetBP_Core_HUD))) AbilityClass))

(event Custom|CancelCast
  ;[0 0 0] CancelCast
  (CallFunction|SRCancelCast)
  (Default|CancelCast (Variables|/Game/xrn/Widgets/UI/WB_HUD.WB_HUD_C|GetWB_CastBar (Variables|/Game/xrn/Blueprints/Core/BP_Core_HUD.BP_Core_HUD_C|GetWB_HUD (Variables|Default|GetBP_Core_HUD)))))

(event Custom|SR_InterruptCast
  ;[0 0 0] CancelCast
  (Default|SRCancelCast (Variables|Default|GetBP_Core_GS)))

(event Custom|InterruptCast
  ;[0 0 0] CancelCast
  (CallFunction|SRInterruptCast)
  (Default|InterruptCast (Variables|/Game/xrn/Widgets/UI/WB_HUD.WB_HUD_C|GetWB_CastBar (Variables|/Game/xrn/Blueprints/Core/BP_Core_HUD.BP_Core_HUD_C|GetWB_HUD (Variables|Default|GetBP_Core_HUD)))))

(event Custom|SR_CancelCast
  ;[0 0 0] CancelCast
  (Default|SRCancelCast (Variables|Default|GetBP_Core_GS)))

(fn ConstructionScript)