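; Core GameMode that tracks connected players and provides player spawning.
; Login, logout and controller-swap events keep PCArray up to date through add and remove helpers, which accept only BP_Core_PC controllers and print an error otherwise.
; SpawnPlayer, not called within this graph, destroys any existing pawn, spawns PlayerCharacterType at a random PlayerStart and possesses it.
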(event EventPostLogin
  (params (NewPlayer :type Player%20Controller%20Object%20Reference))
  ;[1 1 1] Player connection maintainer
  ;;[1 1 1] OnConnect
  (Utilities|AddPCtoList NewPlayer))

(event EventOnSwapPlayerControllers
  (params (OldPC :type Player%20Controller%20Object%20Reference) (NewPC :type Player%20Controller%20Object%20Reference))
  ;[1 1 1] Player connection maintainer
  ;;[1 1 1] OnConnect
  (Utilities|RemovePCtoList OldPC
    (:Success
      (Utilities|AddPCtoList NewPC))))

(event EventOnLogout
  (params (ExitingController :type Controller%20Object%20Reference))
  ;[1 1 1] Player connection maintainer
  ;;[1 1 1] OnDisconnect
  (bind _asplayer_controller (Utilities|Casting|CastToPlayerController ExitingController)
    (:then
      (Utilities|RemovePCtoList _asplayer_controller))
    (:CastFailed
      (CallFunction|PrintError "BP_GM_BaseSetup:Event OnLogout" "Failed to Cast to Player_Controller"))))

(fn ConstructionScript)

(fn SpawnPlayer
  (params (PC :type BP%20Core%20PC%20Object%20Reference))
  (bind _validatedobject (Utilities|IsValidObject (Pawn|GetControlledPawn PC))
    (:IsValid
      (Actor|DestroyActor _validatedobject))
    (:IsNotValid
      _))
  (bind _returnvalue (Game|SpawnActorfromClass (Variables|Default|GetPlayerCharacterType) (Spawn|FindRandomPlayerStart) "Undefined" "MultiplyWithRoot" 0 0))
  (Pawn|Possess PC (.AsPawn (Utilities|Casting|CastToPawn _returnvalue))))

(fn FindRandomPlayerStart
  (bind _outactors (Actor|GetAllActorsOfClass "/Script/Engine.PlayerStart"))
  (return (Transformation|GetActorTransform (Utilities|Array|Get(acopy) _outactors (Math|Random|RandomIntegerinRange 0 (- (Utilities|Array|Length _outactors) 1))))))