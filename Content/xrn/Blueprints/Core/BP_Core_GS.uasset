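; BP_Core_GS is the core game state that coordinates ability spawning, firing, cancelling and destruction.
; SR_SpawnAbility spawns the ability actor, has each BP_Core_PC from PlayerArray spawn a client copy through a macro loop, then starts the cast.
; Firing relays through a multicast event to a dispatcher, while cancel and interrupt both call the cancel-cast dispatcher directly.
; DebugBind attaches print handlers to the ability dispatchers.
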(event Custom|OnAbilityBeginCastDispatcher_Event
  (Development|PrintString "OnAbilityBeginCastDispatcher_Event"))

(event Custom|DebugBind
  (EventDispatchers|BindEventtoOnAbilityBeginCastDispatcher (delegate Custom|OnAbilityBeginCastDispatcher_Event))
  (EventDispatchers|BindEventtoOnAbilityFireDispatcher (delegate Custom|OnAbilityFireDispatcher_Event))
  (EventDispatchers|BindEventtoOnAbilityHitDispatcher (delegate Custom|OnAbilityHitDispatcher_Event))
  (EventDispatchers|BindEventtoOnAbilityOverTimeEffectDispatcher (delegate Custom|OnAbilityOverTimeEffectDispatcher_Event))
  (EventDispatchers|BindEventtoOnAbilityCancelCastDispatcher (delegate Custom|OnAbilityCancelCastDispatcher_Event))
  (EventDispatchers|BindEventtoOnAbilityInterruptCastDispatcher (delegate Custom|OnAbilityInterruptCastDispatcher_Event)))

(event Custom|SR_FireAbility
  ;[0 0 0] Fire Ability
  (CallFunction|MCFireAbility))

(event Custom|MC_FireAbility
  ;[0 0 0] Fire Ability
  (Default|CallOnAbilityFireDispatcher))

(event Custom|OnAbilityFireDispatcher_Event
  (Development|PrintString "OnAbilityFireDispatcher_Event"))

(event Custom|OnAbilityHitDispatcher_Event
  (Development|PrintString "OnAbilityHitDispatcher_Event"))

(event Custom|OnAbilityOverTimeEffectDispatcher_Event
  (Development|PrintString "OnAbilityOverTimeEffectDispatcher_Event"))

(event Custom|SR_DestroyAbility
  (params (Ability%20to%20destroy :type BP%20Ability%20Object%20Reference))
  ;[0 0 0] Destroy Ability
  (bind _validatedobject (Utilities|IsValidObject Ability%20to%20destroy)
    (:IsValid
      (Actor|DestroyActor _validatedobject))))

(event Custom|OnAbilityCancelCastDispatcher_Event
  (Development|PrintString "OnAbilityCancelCastDispatcher_Event"))

(event Custom|OnAbilityInterruptCastDispatcher_Event
  (Development|PrintString "OnAbilityInterruptCastDispatcher_Event"))

(event Custom|SR_SpawnAbility
  (params (AbilityClass :type BP%20Ability%20Class%20Reference) (Instigator :type Pawn%20Object%20Reference))
  ;[0 0 0] Use Ability
  (bind _returnvalue (Game|SpawnActorfromClass AbilityClass (Transformation|GetActorTransform Instigator) "Undefined" "MultiplyWithRoot" 0 Instigator))
  (bind _bp_core_pc (Utilities|ForEachPlayerController)
    (:Loop%20Body
      (Default|OCSpawnClientAbility _bp_core_pc (Transformation|GetActorTransform _returnvalue) (Utilities|GetClass _returnvalue) Instigator))
    (:Completed
      (Default|SRBeginCast _returnvalue))))

(event Custom|SR_InterruptCast
  ;[0 0 0] Interrupt Cast
  (Default|CallOnAbilityCancelCastDispatcher))

(event Custom|SR_CancelCast
  ;[0 0 0] Cancel Cast
  (Default|CallOnAbilityCancelCastDispatcher))

(fn ConstructionScript)