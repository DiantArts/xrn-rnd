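; BP_Core_PS is a PlayerState Blueprint that shows the local player's name in the HUD.
; On BeginPlay it casts player controller 0's HUD to BP_Core_HUD and writes player state 0's name into the WBHUD username text.
; It reads both by index rather than from its own instance, and prints an error if the cast fails.
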(event Custom|OC_SetPlayerNameInHUD
  (bind _asbp_core_hud (Utilities|Casting|CastToBP_Core_HUD (HUD|GetHUD (Game|GetPlayerController 0)))
    (:then
      (Rendering|Components|TextRender|SetText (Variables|/Game/xrn/Widgets/UI/WB_HUD.WB_HUD_C|GetUsername_Text (Variables|/Game/xrn/Blueprints/Core/BP_Core_HUD.BP_Core_HUD_C|GetWB_HUD _asbp_core_hud)) (Utilities|Text|ToText(String) (PlayerState|GetPlayerName (Game|GetPlayerState 0)))))
    (:CastFailed
      (CallFunction|PrintError "BP_Core_PS:BeginPlay" "Failed to cast HUD to BP_Core_HUD"))))

(event EventBeginPlay
  (CallFunction|OCSetPlayerNameinHUD))

(fn ConstructionScript)