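; Client-side ability actor that presents an ability's audio and visual effects from data in its Ability class defaults.
; The construction script adds or reuses an AbilityProjectileComponent for projectile abilities.
; SpawnEffect uses the actor's own audio and particle components for permanent effects, or spawns temporary ones at its location.
; Only cast start triggers effects; setup, fire, impact and hit are stubs with disconnected game-state dispatcher logic, and other events print or are empty.
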(event Custom|OnAbilityDestroy
  (Development|PrintString "Ability Destroyed"))

(event Custom|MC_OnAbilityOverTimeEffectsTick
  (params (AffectedActor :type Object%20Object%20Reference)))

(event Custom|MC_OnAbilityHit
  (params (AffectedActor :type Actor%20Object%20Reference)))

(event Custom|OnAbilityCancelCast
  (Development|PrintString "Ability Canceled"))

(event Custom|OnAbilityInterruptCast
  (Development|PrintString "Ability Interrupted"))

(event Custom|OnAbilityExpire
  (Development|PrintString "Ability Expire"))

(fn ConstructionScript
  (bind _self self)
  (bind _ability (Variables|Default|GetAbility))
  (bind _s_ability_details_projectile_type (Utilities|GetClassDefaults _ability))
  (if (.isprojectile (.S%20Ability%20Details%20Projectile%20Type (Utilities|GetClassDefaults (Variables|Default|GetAbility))))
    ;[1 1 1] Ability Projectile Component
    (bind _component (Utilities|HasComponent "/Game/xrn/Blueprints/Abilities/AbilityComponents/AbilityProjectileComponent.AbilityProjectileComponent_C")
      (:True
        (Default|ConstructComponent (.AsAbility%20Projectile%20Component (Utilities|Casting|CastToAbilityProjectileComponent _component)) _self _s_ability_details_projectile_type))
      (:False
        (bind _returnvalue (AddComponent|AddAbilityProjectileComponent))
        (Default|ConstructComponent _returnvalue _self _s_ability_details_projectile_type)))))

(fn SpawnEffect
  (params (Effect :type F%20Audio%20Visual%20Effects%20Structure))
  (bind _audio (Variables|Default|GetAudio))
  (if (.ispermanent Effect)
    ;[1 1 1] With infinit effect duration
    (bind _validatedobject (Utilities|IsValidObject (.audioeffect Effect))
      (:IsValid
        (Audio|Components|Audio|SetSound _audio _validatedobject))
      (:IsNotValid
        _))
    (Audio|Components|Audio|Play _audio 0.0)
    (bind _validatedobject_2 (Utilities|IsValidObject (.visualeffect Effect))
      (:IsValid
        (Effects|Components|ParticleSystem|SetTemplate (Variables|Default|GetParticleSystem) _validatedobject_2)
        (Transformation|SetWorldScale3D (Variables|Default|GetParticleSystem) (.scale Effect))
        (Transformation|SetWorldRotation (Variables|Default|GetParticleSystem) (.rotation Effect) false false)))
    (else
      ;[1 1 1] With temporary effect
      (bind _validatedobject_3 (Utilities|IsValidObject (.audioeffect Effect))
        (:IsValid
          (Audio|PlaySoundatLocation _validatedobject_3 (Transformation|GetActorLocation) "0, 0, 0" 1.0 1.0 0.0 0 0 0 0))
        (:IsNotValid
          (bind _validatedobject_4 (Utilities|IsValidObject (.visualeffect Effect))
            (:IsValid
              (Effects|SpawnEmitteratLocation _validatedobject_4 (Transformation|GetActorLocation) (.rotation Effect) (.scale Effect)))))))))

(fn OnSetup)

(fn OnBeginCast
  (Development|PrintString "Ability Cast Begon")
  (Helpers|SpawnEffect (.casteffects (.S%20Ability%20Details%20Effects (Utilities|GetClassDefaults (Variables|Default|GetAbility))))))

(fn OnFire)

(fn OnImpact
  (params (Location :type Vector)))

(fn OnHit
  (params (HitActor :type Actor%20Object%20Reference)))