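; Base networked ability actor that runs a data-driven lifecycle: cast, fire, impact, hit, periodic effect, expire or destroy.
; MC_EventBinder events route each stage to server (SR_) gameplay or client (CL_) effects, with several client handlers still stubs.
; Optional projectile, ground and damage components handle movement and damage.
; The root sphere detects first valid impact, then resizes for AoE hits and timed periodic scans, filtered by caster/character rules.
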(event OnComponentBeginOverlap(AbilityRoot)
  (params (OverlappedComponent :type Primitive%20Component%20Object%20Reference) (OtherActor :type Actor%20Object%20Reference) (OtherComp :type Primitive%20Component%20Object%20Reference) (OtherBodyIndex :type Integer) (bFromSweep :type Boolean) (SweepResult :type Hit%20Result%20Structure%20%28by%20ref%29))
  ;[0 0 0] Hit events
  (Utilities|IsServer
    (:true
      (if (not (== OtherActor (Game|GetInstigator))) ; Is the other actor the castor
        (bind _value (ServerAbilityFlow|SRIsValidImpact OtherActor))
        (if _value
          (CallFunction|MCEventBinderImpact OtherActor))))))

(event Custom|OnAbilityDestroy
  (Development|PrintString "Ability Destroyed"))

(event Custom|OnPeriodicEffectsTick
  (params (AffectedActor :type Object%20Object%20Reference))
  (Development|PrintText (Utilities|Text|FormatText "Ability {abilityName}'s tick hits {targetName}" (.name (Variables|AbilitySettings|GetS%20Ability%20Details%20Meta%20Data)) (Utilities|GetDisplayName AffectedActor))))

(event Custom|OnAbilityHit
  (params (AffectedActor :type Actor%20Object%20Reference))
  (Development|PrintText (Utilities|Text|FormatText "Ability {abilityName} hits {targetName}" (.name (Variables|AbilitySettings|GetS%20Ability%20Details%20Meta%20Data)) (Utilities|GetDisplayName AffectedActor))))

(event Custom|OnCancelCast
  (Development|PrintString "Ability Canceled"))

(event Custom|OnInterruptCast
  (Development|PrintString "Ability Interrupted"))

(event Custom|OnAbilityExpire
  (Development|PrintString "Ability Expire"))

(event Collision|EventHit
  (params (MyComp :type Primitive%20Component%20Object%20Reference) (Other :type Actor%20Object%20Reference) (OtherComp :type Primitive%20Component%20Object%20Reference) (bSelfMoved :type Boolean) (HitLocation :type Vector :default "0, 0, 0") (HitNormal :type Vector :default "0, 0, 0") (NormalImpulse :type Vector :default "0, 0, 0") (Hit :type Hit%20Result%20Structure%20%28by%20ref%29))
  ;[0 0 0] Hit events
  (Utilities|IsServer
    (:true
      (if (.doesaffectobjects (Variables|AbilitySettings|GetS%20Ability%20Details%20Hit))
        (bind _value (ServerAbilityFlow|SRIsValidImpact Other))
        (if _value
          (CallFunction|MCEventBinderImpact Other))))))

(event Custom|MC_EventBinder_Fire
  (Utilities|IsServer
    (:true
      (ServerAbilityFlow|SRFire))
    (:false
      (ClientAbilityFlow|CLFire))))

(event Custom|MC_EventBinder_BeginCast
  (Utilities|IsServer
    (:true
      (ServerAbilityFlow|SRBeginCast))
    (:false
      (ClientAbilityFlow|CLBeginCast))))

(event Custom|MC_EventBinder_Expire
  (Utilities|IsServer
    (:true
      (ServerAbilityFlow|SRExpire))
    (:false
      (ClientAbilityFlow|CLExpire))))

(event Custom|MC_EventBinder_impact
  (params (HitActor :type Actor%20Object%20Reference))
  (Utilities|IsServer
    (:true
      (ServerAbilityFlow|SRImpact HitActor))
    (:false
      (ClientAbilityFlow|CLImpact))))

(event Custom|MC_EventBinder_Hit
  (params (HitActor :type Actor%20Object%20Reference))
  (Utilities|IsServer
    (:true
      (ServerAbilityFlow|SRHit HitActor))
    (:false
      (ClientAbilityFlow|CLHit HitActor))))

(event Custom|MC_EventBinder_PeriodicEffect
  (params (HitActor :type Actor%20Object%20Reference))
  (Utilities|IsServer
    (:true
      (ServerAbilityFlow|SRPeriodicEffect HitActor))
    (:false
      (ClientAbilityFlow|CLPeriodicEffect))))

(event Custom|MC_EventBinder_Destroy
  (Utilities|IsServer
    (:true
      (ServerAbilityFlow|SRDestroy))
    (:false
      (ClientAbilityFlow|CLDestroy))))

(event Custom|MC_EventBinder_Cancel
  (Utilities|IsServer
    (:true
      (ServerAbilityFlow|SRCancel))
    (:false
      (ClientAbilityFlow|CLCancel))))

(event Custom|MC_EventBinder_Interrupt
  (Utilities|IsServer
    (:true
      (ServerAbilityFlow|SRInterrupt))
    (:false
      (ClientAbilityFlow|CLInterrupt))))

(fn ConstructionScript
  (bind _self self)
  (bind _s_ability_details_projectile_type (Variables|AbilitySettings|GetS%20Ability%20Details%20Projectile%20Type))
  (if (.isprojectile (Variables|AbilitySettings|GetS%20Ability%20Details%20Projectile%20Type))
    ;[1 1 1] Ability Projectile Component
    (bind _component (Utilities|HasComponent "/Game/xrn/Blueprints/Abilities/AbilityComponents/AbilityProjectileComponent.AbilityProjectileComponent_C")
      (:True
        (Default|ConstructComponent (.AsAbility%20Projectile%20Component (Utilities|Casting|CastToAbilityProjectileComponent _component)) _self _s_ability_details_projectile_type))
      (:False
        (bind _returnvalue (AddComponent|AddAbilityProjectileComponent))
        (Default|ConstructComponent _returnvalue _self _s_ability_details_projectile_type)))
    (Components|Sphere|SetSphereRadius (Variables|Default|GetAbilityRoot) (.hitsphereprojectileradius (Variables|AbilitySettings|GetS%20Ability%20Details%20Projectile%20Type)) true)))

(fn SpawnEffect
  (params (Effect :type F%20Audio%20Visual%20Effects%20Structure))
  (bind _audio (Variables|Default|GetAudio))
  (if (.ispermanent Effect)
    ;[1 1 1] With infinit effect duration
    (bind _validatedobject (Utilities|IsValidObject (.audioeffect Effect))
      (:IsValid
        (Audio|Components|Audio|SetSound _audio _validatedobject))
      (:IsNotValid
        _))
    (Audio|Components|Audio|Play _audio 0.0)
    (bind _validatedobject_2 (Utilities|IsValidObject (.visualeffect Effect))
      (:IsValid
        (Effects|Components|ParticleSystem|SetTemplate (Variables|Default|GetParticleSystem) _validatedobject_2)
        (Transformation|SetWorldScale3D (Variables|Default|GetParticleSystem) (.scale Effect))
        (Transformation|SetWorldRotation (Variables|Default|GetParticleSystem) (.rotation Effect) false false)))
    (else
      ;[1 1 1] With temporary effect
      (bind _validatedobject_3 (Utilities|IsValidObject (.audioeffect Effect))
        (:IsValid
          (Audio|PlaySoundatLocation _validatedobject_3 (Transformation|GetActorLocation) "0, 0, 0" 1.0 1.0 0.0 0 0 0 0))
        (:IsNotValid
          (bind _validatedobject_4 (Utilities|IsValidObject (.visualeffect Effect))
            (:IsValid
              (Effects|SpawnEmitteratLocation _validatedobject_4 (Transformation|GetActorLocation) (.rotation Effect) (.scale Effect)))))))))

(fn UseCorrectAbilityProjectileComponent
  (Utilities|FlowControl|Sequence
    (:then_0
      ;[1 1 1] Ability Projectile Component
      (bind _component (Utilities|HasComponent "/Game/xrn/Blueprints/Abilities/AbilityComponents/AbilityProjectileComponent.AbilityProjectileComponent_C")
        (:True
          (Default|DoFireAbility (.AsAbility%20Projectile%20Component (Utilities|Casting|CastToAbilityProjectileComponent _component)))
          (return false))))
    (:then_1
      ;[1 1 1] Ability Projectile Ground Component
      (Utilities|HasComponent "/Game/xrn/Blueprints/Abilities/AbilityComponents/AbilityProjectileGroundComponent.AbilityProjectileGroundComponent_C"
        (:True
          (return true))))))

(fn SRUse
  (CallFunction|MCEventBinderBeginCast))

(fn SRBeginCast
  ;[1 1 1] Setup
  (Utilities|IsServerCheck "BP_Ability:SR_BeginCast" true
    (:true
      (bind _asbp_core_gs (Utilities|Casting|CastToBP_Core_GS (Game|GetGameState))
        (:then
          (Variables|Helpers|SetBP_Core_GS _asbp_core_gs)
          (if (> (.casttime (Variables|AbilitySettings|GetS%20Ability%20Details%20Cast)) 0.0)
            ;[1 1 1] CastAbility
            (bind _returnvalue (Utilities|Time|SetTimerbyEvent (EventDispatchers|CreateEvent :!event Custom|MC_EventBinder_Fire) (.casttime (Variables|AbilitySettings|GetS%20Ability%20Details%20Cast))))
            (Variables|Default|SetCastTimerHandle _returnvalue)
            (else
              ;[1 1 1] Fire instantly if no cast
              (CallFunction|MCEventBinderFire))))
        (:CastFailed
          (CallFunction|PrintError "BP_ClientAbility:OnSetup" "Cast to BP_Core_GS failed"))))))

(fn SRFire
  (Utilities|IsServerCheck "BP_Ability:SR_Fire" true
    (:true
      (bind _shoulddirectlyhit (ServerAbilityFlow|Helpers|UseCorrectAbilityProjectileComponent))
      (LocalVariables|SetShouldDirectlyHit _shoulddirectlyhit)
      (Transformation|DetachFromActor "KeepWorld" "KeepWorld" "KeepWorld")
      (if (LocalVariables|GetShouldDirectlyHit)
        ;[1 1 1] Has instant impact?
        (CallFunction|MCEventBinderImpact)))))

(fn SRImpact
  (params (HitActor :type Actor%20Object%20Reference))
  (Utilities|IsServerCheck "BP_Ability:SR_Impact" true
    (:true
      (Utilities|FlowControl|Sequence
        (:then_0
          ;[1 1 1] Ability Projectile Components
          ;;[1 1 1] Ability Projectile Ground Component
          (bind _component (Utilities|HasComponent "/Game/xrn/Blueprints/Abilities/AbilityComponents/AbilityProjectileGroundComponent.AbilityProjectileGroundComponent_C")
            (:True
              (Default|DoFireAbility (.AsAbility%20Projectile%20Ground%20Component (Utilities|Casting|CastToAbilityProjectileGroundComponent _component)) self))))
        (:then_1
          ;;[1 1 1] Ability Projectile Component
          (bind _component_2 (Utilities|HasComponent "/Game/xrn/Blueprints/Abilities/AbilityComponents/AbilityProjectileComponent.AbilityProjectileComponent_C")
            (:True
              (Default|DoImpactAbility (.AsAbility%20Projectile%20Component (Utilities|Casting|CastToAbilityProjectileComponent _component_2))))))
        (:then_2
          ;[1 1 1] OnAbilityHitDispatcher
          (Components|Sphere|SetSphereRadius (Variables|Default|GetAbilityRoot) (.hitsphereradius (Variables|AbilitySettings|GetS%20Ability%20Details%20Hit)) true)
          (if (.isaoe (Variables|AbilitySettings|GetS%20Ability%20Details%20Hit))
            ;;[1 1 1] AoE effect
            (for _array_element (Collision|GetOverlappingActors (Variables|Default|GetAbilityRoot) "/Script/Engine.Pawn" :!class /Script/Engine.PrimitiveComponent)
              (CallFunction|MCEventBinderHit _array_element))
            (else
              ;;[1 1 1] Single target Effect
              (CallFunction|MCEventBinderHit HitActor))))
        (:then_3
          ;[1 1 1] Has effects over time
          (if (<= (.abilityduration (Variables|AbilitySettings|GetS%20Ability%20Details%20Hit)) 0.0)
            ;[1 1 1] Destroy the actor if it was a single hit
            (CallFunction|MCEventBinderDestroy)
            (else
              ;[1 1 1] Set up Over time events
              (Utilities|FlowControl|Sequence
                (:then_0
                  (Utilities|Time|SetTimerbyEvent (EventDispatchers|CreateEvent :!event Custom|MC_EventBinder_Expire) (.abilityduration (Variables|AbilitySettings|GetS%20Ability%20Details%20Hit))))
                (:then_1
                  (ServerAbilityFlow|SRScanforPeriodicEffect)
                  (Utilities|Time|SetTimerbyEvent (EventDispatchers|CreateEvent :!event SRScanforPeriodicEffect) (.effectfrequency (Variables|AbilitySettings|GetS%20Ability%20Details%20Hit)) true))))))))))

(fn SRIsValidImpact
  (params (HitActor :type Actor%20Object%20Reference))
  (Utilities|IsServerCheck "BP_Ability:SR_IsValidImpact" true
    (:true
      (bind _validatedobject (Utilities|IsValidObject HitActor)
        (:IsValid
          (Utilities|IsActorAffectedbyAbility _validatedobject
            (:True
              (if (Variables|Helpers|GetIsFirstAbilityImpactBool)
                (Variables|Helpers|SetIsFirstAbilityImpactBool false)
                (return true)
                (else
                  (return false))))
            (:False
              (return false))))
        (:IsNotValid
          (return false))))
    (:false
      (return false))))

(fn SRHit
  (params (HitActor :type Actor%20Object%20Reference))
  (Utilities|IsServerCheck "BP_Ability:SR_Hit" true
    (:true
      ;[1 1 1] Ability Damage Component
      (bind _component (Utilities|HasComponent "/Game/xrn/Blueprints/Abilities/AbilityComponents/AbilityDamageComponent.AbilityDamageComponent_C")
        (:True
          (Default|ComponentDoDamage (.AsAbility%20Damage%20Component (Utilities|Casting|CastToAbilityDamageComponent _component)) self HitActor))))))

(fn SRScanforPeriodicEffect
  (for _array_element (Collision|GetOverlappingActors (Variables|Default|GetAbilityRoot) "/Script/Engine.Pawn" :!class /Script/Engine.PrimitiveComponent)
    (CallFunction|MCEventBinderPeriodicEffect _array_element)))

(fn SRPeriodicEffect
  (params (HitActor :type Actor%20Object%20Reference))
  (Utilities|IsServerCheck "BP_Ability:SR_Expire" true
    (:true
      (bind _validatedobject (Utilities|IsValidObject HitActor)
        (:IsValid
          (Utilities|IsActorAffectedbyAbility _validatedobject
            (:True
              ;[1 1 1] Ability Damage Over Time Component
              (bind _component (Utilities|HasComponent "/Game/xrn/Blueprints/Abilities/AbilityComponents/AbilityDamageOverTimeComponent.AbilityDamageOverTimeComponent_C")
                (:True
                  (Default|ComponentDoDamageOnce (.AsAbility%20Damage%20Over%20Time%20Component (Utilities|Casting|CastToAbilityDamageOverTimeComponent _component)) self HitActor))))))))))

(fn SRExpire
  (Utilities|IsServerCheck "BP_Ability:SR_Expire" true
    (:true
      (CallFunction|MCEventBinderDestroy))))

(fn CLBeginCast
  ;[0 0 0] Setup
  (Utilities|IsServerCheck "BP_Ability:CL_Setup" false
    (:false
      (bind _asbp_core_gs (Utilities|Casting|CastToBP_Core_GS (Game|GetGameState))
        (:then
          (Variables|Helpers|SetBP_Core_GS _asbp_core_gs)
          (if (> (.casttime (Variables|AbilitySettings|GetS%20Ability%20Details%20Cast)) 0.0)
            ;[0 0 0] Do Cast
            (Development|PrintString "Ability Cast Begon")
            (ClientAbilityFlow|Helpers|SpawnEffect (.casteffects (Variables|AbilitySettings|GetS%20Ability%20Details%20Effects)))
            (else
              ;[0 0 0] Fire instantly if no cast time
              (ClientAbilityFlow|CLFire))))
        (:CastFailed
          (CallFunction|PrintError "BP_Ability:CL_Setup" "Cast to BP_Core_GS failed"))))))

(fn CLFire
  (Utilities|IsServerCheck "BP_Ability:CL_Fire" false
    (:false
      (Development|PrintString "Ability Fired")
      (Transformation|DetachFromActor "KeepWorld" "KeepWorld" "KeepWorld")
      (bind _component (Utilities|HasComponent "/Game/xrn/Blueprints/Abilities/AbilityComponents/AbilityProjectileComponent.AbilityProjectileComponent_C")
        (:True
          (Default|DoFireAbility (.AsAbility%20Projectile%20Component (Utilities|Casting|CastToAbilityProjectileComponent _component)))
          (ClientAbilityFlow|Helpers|SpawnEffect (.projectileeffects (Variables|AbilitySettings|GetS%20Ability%20Details%20Effects))))))))

(fn CLImpact
  (bind _s_ability_details_effects (Variables|AbilitySettings|GetS%20Ability%20Details%20Effects))
  (Utilities|IsServerCheck "BP_Ability:CL_Impact" false
    (:false
      (Development|PrintString "Ability Impact")
      ;[1 1 1] Ability Projectile Component
      (bind _component (Utilities|HasComponent "/Game/xrn/Blueprints/Abilities/AbilityComponents/AbilityProjectileComponent.AbilityProjectileComponent_C")
        (:True
          (Default|DoImpactAbility (.AsAbility%20Projectile%20Component (Utilities|Casting|CastToAbilityProjectileComponent _component)))
          ;[1 1 1] OnImpact Visual&Audio
          (ClientAbilityFlow|Helpers|SpawnEffect (.impacteffects _s_ability_details_effects))
          (ClientAbilityFlow|Helpers|SpawnEffect (.abilityeffects _s_ability_details_effects)))))))

(fn CLHit
  (params (HitActor :type Actor%20Object%20Reference))
  (Utilities|IsServerCheck "BP_Ability:CL_Hit" false
    (:false
      (ClientAbilityFlow|Helpers|SpawnEffect (.hiteffects (Variables|AbilitySettings|GetS%20Ability%20Details%20Effects))))))

(fn CLPeriodicEffect
  (Utilities|IsServerCheck "BP_Ability:SR_PeriodicEffect" false))

(fn CLExpire
  (Utilities|IsServerCheck "BP_Ability:SR_Expire" false))

(fn CLCancel
  (Utilities|IsServerCheck "BP_Ability:CL_Cancel" false))

(fn CLInterrupt
  (Utilities|IsServerCheck "BP_Ability:CL_Interrupt" false))

(fn CLDestroy
  (Utilities|IsServerCheck "BP_Ability:SR_Destroy" false))

(fn SRCancel
  (Utilities|IsServerCheck "BP_Ability:SR_Cancel" true
    (:true
      (CallFunction|MCEventBinderDestroy))))

(fn SRInterrupt
  (Utilities|IsServerCheck "BP_Ability:SR_Interrupt" true
    (:true
      (CallFunction|MCEventBinderDestroy))))

(fn SRDestroy
  (Actor|DestroyActor))