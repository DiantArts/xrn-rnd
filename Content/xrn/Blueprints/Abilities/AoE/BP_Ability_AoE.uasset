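; Area-of-effect ability Blueprint that handles placement on fire and damage-over-time ticks.
; On fire it zeroes its rotation and, when grounded, traces down from player 0 to snap onto the surface below.
; Each effect tick loops over actors overlapping AbilityRoot, calling ApplyDamage with no damaged actor wired; the instigator only qualifies when DoesAffectObjects is set.
; Hits defer to the parent, while begin, cancel and interrupt cast events are empty.
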(event EventOnAbilityFire
  (bind _returnvalue (Game|GetPlayerCharacter 0))
  (bind _returnvalue_2 (Transformation|GetActorLocation _returnvalue))
  (Transformation|SetActorRotation "0, 0, 0")
  (if (Variables|AbilitySettings|Aoesettings|GetIsGrounded)
    (bind (_outhit _returnvalue_3) (Collision|LineTraceByChannel _returnvalue_2 (+ _returnvalue_2 "0.000000,0.000000,-10000.000000") "TraceTypeQuery1" false (Utilities|Array|MakeArray _returnvalue) "None"))
    (if _returnvalue_3
      (Transformation|SetActorLocation (.location _outhit) false false))))

(event EventOnAbilityHit
  (params (AffectedActor :type Actor%20Object%20Reference))
  (|CallParentFunction AffectedActor))

(event EventOnAbilityOverTimeEffectsTick
  (params (AffectedActor :type Object%20Object%20Reference))
  ;[1 1 1] Damage loop
  (for _array_element (Collision|GetOverlappingActors (Variables|Default|GetAbilityRoot) 0 :!class /Script/Engine.PrimitiveComponent)
    (if (== _array_element (Game|GetInstigator)) ; Is player
      (if (.doesaffectobjects (Variables|Default|GetS%20Ability%20Details%20Hit)) ; Is affecting player
        (Game|Damage|ApplyDamage 0 (.damage (Variables|Default|GetS%20Ability%20Details%20Hit)) (Game|GetInstigatorController) self :!label _label)
        (Development|PrintString "DoT applied"))
      (else
        (goto _label)))))

(event EventOnAbilityCancelCast)

(event EventOnAbilityInterruptCast)

(event EventOnAbilityBeginCast)

(fn ConstructionScript
  (|CallParentFunction))